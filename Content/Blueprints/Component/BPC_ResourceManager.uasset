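; BPC_ResourceManager is a component meant to track the current amount and maximum capacity of each resource type.
; On BeginPlay it loops over every DT_Resources row to fill the CurrentAmount and MaxCapacity maps with default and max values.
; It then calls the OnResourcesInitialized dispatcher between debug prints.
; The add, consume, get-amount and has-enough functions are empty stubs, and Tick is unused.
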(event `self.ReceiveBeginPlay`
  (bind _outrownames (`DataTableFunctionLibrary.GetDataTableRowNames` "/Game/Blueprints/Data/DT_Resources.DT_Resources"))
  (for _array_element _outrownames
    (bind _returnvalue (`|GetDataTableRow` "/Game/Blueprints/Data/DT_Resources.DT_Resources" _array_element)
      (:`then`
        (bind (_resourcetype _defaultamount _maxamount) (break `/Game/Blueprints/Data/STR_ResourceSet` _returnvalue))
        (`BlueprintMapLibrary.Map_Add` (`self.CurrentAmount`) _resourcetype _defaultamount)
        (`BlueprintMapLibrary.Map_Add` (`self.MaxCapacity`) _resourcetype _maxamount))))
  (`KismetSystemLibrary.PrintString` "Je déclange un event")
  (`self.OnResourcesInitialized`)
  (`KismetSystemLibrary.PrintString` "Done"))

(fn `AddResource`)

(fn `ConsumeResource`)

(fn `GetResourceAmount`)

(fn `HasEnoughResources`)