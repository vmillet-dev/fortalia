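; Player controller for a fixed-angle 3/4 orthographic camera, driving BP_Pawn as a floating view through Enhanced Input.
; Movement remaps input axes into diagonals relative to control yaw, while dragging offsets the pawn by the viewport mouse delta rotated by camera yaw.
; Zoom is clamped and passed to the pawn's ZoomModifier, and reset restores the width cached at BeginPlay.
; Select-object and pause inputs are empty stubs.
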(event `EnhancedInput|/Game/Blueprints/Input/Actions/IA_CameraDrag`
  (params (ActionValue :type "Vector2D Structure") (ElapsedSeconds :type "Float (double-precision)") (TriggeredSeconds :type "Float (double-precision)") (InputAction :type "InputAction Object Reference" :default "/Game/Blueprints/Input/Actions/IA_CameraDrag.IA_CameraDrag"))
  ; Camera logic
  ;; Camera draggig
  (:`Triggered`
    (bind _returnvalue (`WidgetLayoutLibrary.GetMousePositionOnViewport`))
    (set `self.GetNewMousePosition` _returnvalue)
    (`self.DragCameraView`)
    (set `self.GetLastMousePosition` (`self.GetNewMousePosition`)))
  (:`Started`
    (bind _returnvalue_2 (`WidgetLayoutLibrary.GetMousePositionOnViewport`))
    (set `self.GetLastMousePosition` _returnvalue_2)))

(event `EnhancedInput|/Game/Blueprints/Input/Actions/IA_CameraMove`
  (params (ActionValue :type "Vector2D Structure") (ElapsedSeconds :type "Float (double-precision)") (TriggeredSeconds :type "Float (double-precision)") (InputAction :type "InputAction Object Reference" :default "/Game/Blueprints/Input/Actions/IA_CameraMove.IA_CameraMove"))
  (bind (_returnvalue_roll _returnvalue_pitch _returnvalue_yaw) (`KismetMathLibrary.BreakRotator` (`self.GetControlRotation`)))
  (bind (_returnvalue_roll_2 _returnvalue_pitch_2 _returnvalue_yaw_2) (`KismetMathLibrary.BreakRotator` (`self.GetControlRotation`)))
  (bind _controlledpawn (`self.ControlledPawn`))
  ; Camera logic
  ;; Spectator Pawn Movement - our pawn is essentially a floating fixed angle camera. Because our view is 3/4, we're actually moving diagonally when it looks like we're moving straight
  (:`Triggered`
    (`Pawn.AddMovementInput` _controlledpawn (`KismetMathLibrary.GetForwardVector` (`KismetMathLibrary.MakeRotator` _returnvalue_roll 0.0 _returnvalue_yaw)) (+ ActionValue_X ActionValue_Y) false)
    (`Pawn.AddMovementInput` _controlledpawn (`KismetMathLibrary.GetRightVector` (`KismetMathLibrary.MakeRotator` 0.0 0.0 _returnvalue_yaw_2)) (- ActionValue_X ActionValue_Y) false)))

(event `self.ReceiveBeginPlay`
  (`|ExecutionSequence`
    (:`then_0`
      ; Get Starting Orthographic Zoom
      (bind _asbp_pawn (cast `/Game/Blueprints/Core/BP_Pawn` (`self.K2_GetPawn`)))
      (bind _orthowidth (`CameraComponent.OrthoWidth` (`/Game/Blueprints/Core/BP_Pawn.Camera` _asbp_pawn)))
      (set `self.CurrentZoom` _orthowidth)
      (set `self.ControlledPawn` _asbp_pawn)
      (set `self.DefaultZoom` _orthowidth))
    (:`then_1`
      (`EnhancedInputSubsystemInterface.AddMappingContext` (subsystem `EnhancedInputLocalPlayerSubsystem`) "/Game/Blueprints/Input/IMC_Inputs.IMC_Inputs" 0 (struct)))))

(event `EnhancedInput|/Game/Blueprints/Input/Actions/IA_CameraZoom`
  (params (ActionValue :type "Float (double-precision)") (ElapsedSeconds :type "Float (double-precision)") (TriggeredSeconds :type "Float (double-precision)") (InputAction :type "InputAction Object Reference" :default "/Game/Blueprints/Input/Actions/IA_CameraZoom.IA_CameraZoom"))
  ; Camera logic
  ;; Zoom
  (:`Triggered`
    (bind _result (`/Engine/EditorBlueprintResources/StandardMacros.NegateFloat` ActionValue)
      (:`  `
        (bind _output_get (set `self.CurrentZoom` (`KismetMathLibrary.FClamp` (+ (* _result 100.0) (`self.CurrentZoom`)) 1000.0 4000.0)))
        (`/Game/Blueprints/Core/BP_Pawn.ZoomModifier` (`self.ControlledPawn`) _output_get)))))

(event `EnhancedInput|/Game/Blueprints/Input/Actions/IA_CameraReset`
  (params (ActionValue :type Boolean) (ElapsedSeconds :type "Float (double-precision)") (TriggeredSeconds :type "Float (double-precision)") (InputAction :type "InputAction Object Reference" :default "/Game/Blueprints/Input/Actions/IA_CameraReset.IA_CameraReset"))
  ; Camera logic
  ;; Zoom
  (:`Triggered`
    (bind _output_get (set `self.CurrentZoom` (`self.DefaultZoom`)))
    (`/Game/Blueprints/Core/BP_Pawn.ZoomModifier` (`self.ControlledPawn`) _output_get)))

(event `EnhancedInput|/Game/Blueprints/Input/Actions/IA_SelectObject`
  (params (ActionValue :type Boolean) (ElapsedSeconds :type "Float (double-precision)") (TriggeredSeconds :type "Float (double-precision)") (InputAction :type "InputAction Object Reference" :default "/Game/Blueprints/Input/Actions/IA_SelectObject.IA_SelectObject")))

(event `EnhancedInput|/Game/Blueprints/Input/Actions/IA_TogglePause`
  (params (ActionValue :type Boolean) (ElapsedSeconds :type "Float (double-precision)") (TriggeredSeconds :type "Float (double-precision)") (InputAction :type "InputAction Object Reference" :default "/Game/Blueprints/Input/Actions/IA_TogglePause.IA_TogglePause")))

(fn `DragCameraView`
  (bind (_returnvalue_x _returnvalue_y) (`KismetMathLibrary.BreakVector2D` (- (`self.GetNewMousePosition`) (`self.GetLastMousePosition`))))
  (bind (_relativerotation_roll _relativerotation_pitch _relativerotation_yaw) (`KismetMathLibrary.BreakRotator` (`SceneComponent.RelativeRotation` (`/Game/Blueprints/Core/BP_Pawn.Camera` (`self.ControlledPawn`)))))
  (bind _vector3dcameraparameter_value (break `Vector3dCameraParameter` (make `Vector3dCameraParameter` (`KismetMathLibrary.MakeVector` _returnvalue_y (* _returnvalue_x -1.0)))))
  (`self.K2_AddActorWorldOffset` (`self.ControlledPawn`) (`KismetMathLibrary.GreaterGreater_VectorRotator` _vector3dcameraparameter_value (`KismetMathLibrary.MakeRotator` 0.0 0.0 _relativerotation_yaw)) false false))

(fn `UserConstructionScript`)